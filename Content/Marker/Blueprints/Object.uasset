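; Marker target object that can toggle itself as a current objective on the player's HUD.
; The SetObjective event gets the first player's HUD as BP_Marker and reads its CurrentObjective array.
; It adds itself if absent or removes itself if present, then assigns the array back to the HUD.
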(event `/Game/Marker/Blueprints/BP_ObjectiveMarker_Interface.Set Objective`
  (bind _returnvalue (`KismetArrayLibrary.Array_Find` (`self.Array`) self))
  (bind _asbp_marker (cast `/Game/Marker/Blueprints/BP_Marker` (`PlayerController.GetHUD` (`GameplayStatics.GetPlayerController` 0))))
  (set `self.Array` (`/Game/Marker/Blueprints/BP_Marker.CurrentObjective` _asbp_marker))
  (if (== _returnvalue -1)
    (`KismetArrayLibrary.Array_Add` (`self.Array`) self)
    (else
      (`KismetArrayLibrary.Array_Remove` (`self.Array`) _returnvalue)))
  (bind _asbp_marker_2 (cast `/Game/Marker/Blueprints/BP_Marker` (`PlayerController.GetHUD` (`GameplayStatics.GetPlayerController` 0))))
  (set `/Game/Marker/Blueprints/BP_Marker.CurrentObjective` (`self.Array`) _asbp_marker_2))

(fn `UserConstructionScript`)